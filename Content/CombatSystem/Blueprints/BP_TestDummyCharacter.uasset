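; Test dummy character for the combat system that takes point damage and reacts to hits.
; On BeginPlay it initializes its StatComponent, spawns and equips each starting equipment actor, and prints a current stat value.
; Point damage feeds into the StatComponent and plays impact sound and particles at the hit location.
; If a hit reaction is allowed, it also plays a react montage and changes state through the StateManagerComponent.
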(event `self.ReceiveBeginPlay`
  (`/Game/CombatSystem/Blueprints/Components/AC_StatComponent.InitializeStats` (`self.StatComponent`))
  (for _array_element (`self.StartingEquipment`)
    (bind _returnvalue (`|SpawnActorFromClass` _array_element (`self.GetTransform`) "Undefined" "MultiplyWithRoot" self self))
    (`/Game/CombatSystem/Blueprints/Actors/BP_BaseEquippable.OnEquipped` _returnvalue))
  (`KismetSystemLibrary.PrintString` (`KismetStringLibrary.Conv_DoubleToString` (`/Game/CombatSystem/Blueprints/Components/AC_StatComponent.GetCurrentStatValue` (`self.StatComponent`) "NewEnumerator3"))))

(event `self.ReceivePointDamage`
  (params (Damage :type "Float (single-precision)") (DamageType :type "DamageType Object Reference") (HitLocation :type "Vector Structure") (HitNormal :type "Vector Structure") (HitComponent :type "PrimitiveComponent Object Reference") (BoneName :type Name) (ShotFromDirection :type "Vector Structure") (InstigatedBy :type "Controller Object Reference") (DamageCauser :type "Actor Object Reference") (HitInfo :type "HitResult Structure (by ref)"))
  ;[0.3467 1 0.3515] Damage
  (`/Game/CombatSystem/Blueprints/Components/AC_StatComponent.TakeDamage` (`self.StatComponent`) Damage)
  (`GameplayStatics.PlaySoundAtLocation` "/Game/CombatSystem/CourseFiles/SoundFX/Gruntling/A_Guardian_Impact01_Cue.A_Guardian_Impact01_Cue" HitLocation (struct) 1.0 1.0 0.0 null null null null)
  (`GameplayStatics.SpawnEmitterAtLocation` "/Game/InfinityBladeEffects/Effects/FX_Combat_Base/Impact/P_Impact_Player_Strong.P_Impact_Player_Strong" HitLocation (struct) (0.5 0.5 0.5))
  (if (`self.CanReceiveHitReaction`)
    (`self.PlayAnimMontage` "/Game/CombatSystem/CourseFiles/Animations/HitReactions/AM_Standing_React_Large_Front_Montage.AM_Standing_React_Large_Front_Montage")
    (`/Game/CombatSystem/Blueprints/Components/AC_StateManagerComponent.SetState` (`self.StateManagerComponent`) "NewEnumerator5")))

(fn `UserConstructionScript`
  (`parent.UserConstructionScript`))