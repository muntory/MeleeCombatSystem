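; AN_ToggleCombat is an animation notify that switches a character in or out of combat at a point in an animation.
; It finds the owner's AC_CombatComponent and, if its main weapon is valid, attaches that weapon to the hand or attach socket according to the EnableCombat flag.
; It then passes the same flag to the component's SetCombatEnable.
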(fn `Received_Notify`
  (params (MeshComp :type "SkeletalMeshComponent Object Reference") (Animation :type "AnimSequenceBase Object Reference") (EventReference :type "AnimNotifyEventReference Structure (by ref)"))
  (returns (ReturnValue :type Boolean))
  (bind _returnvalue (`Actor.GetComponentByClass` (`ActorComponent.GetOwner` MeshComp) "/Game/CombatSystem/Blueprints/Components/AC_CombatComponent.AC_CombatComponent_C"))
  (bind _returnvalue_2 (`/Game/CombatSystem/Blueprints/Components/AC_CombatComponent.GetMainWeapon` _returnvalue))
  (`/Engine/EditorBlueprintResources/StandardMacros.IsValid` _returnvalue_2
    (:`Is Valid`
      (`/Game/CombatSystem/Blueprints/Actors/BP_BaseEquippable.AttachActor` _returnvalue_2 (select `bool` (`self.bEnableCombat`) :`false` (`/Game/CombatSystem/Blueprints/Actors/BP_BaseEquippable.Attach Socket Name` _returnvalue_2) :`true` (`/Game/CombatSystem/Blueprints/Actors/BP_BaseWeapon.HandSocketName` _returnvalue_2)))
      (`/Game/CombatSystem/Blueprints/Components/AC_CombatComponent.SetCombatEnable` _returnvalue (`self.bEnableCombat`))
      (return true))
    (:`Is Not Valid`
      (return false))))