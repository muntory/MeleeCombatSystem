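; Actor component for the combat system that holds an owner's stats, such as Health, Stamina and Armor, in maps keyed by stat type.
; Writes clamp to BaseStats limits, then broadcast an update carrying the unclamped value.
; TakeDamage applies armor-scaled damage to Health and sets the owner's state manager to Dead at zero.
; StartRegen restarts stamina regeneration after a retriggerable delay, using a looping timer that clears at max.
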(event `StartRegen`
  (params (StatType :type "/Game/CombatSystem/Blueprints/Enum/E_Stat Enum" :default "NewEnumerator0"))
  (switch `/Game/CombatSystem/Blueprints/Enum/E_Stat` StatType
    (:`NewEnumerator2`
      (`KismetSystemLibrary.K2_ClearTimer` null "RegenStamina")
      (`KismetSystemLibrary.RetriggerableDelay` 1.5)
      (`KismetSystemLibrary.K2_SetTimer` null "RegenStamina" 0.1 true))))

(fn `AddCurrentStatValue`
  (params (Stat :type "/Game/CombatSystem/Blueprints/Enum/E_Stat Enum" :default "NewEnumerator0") (Value :type "Float (double-precision)"))
  (`self.SetCurrentStatValue` Stat (+ Value (`BlueprintMapLibrary.Map_Find` (`self.CurrentStats`) Stat))))

(fn `GetCurrentStatValue`
  (params (Key :type "/Game/CombatSystem/Blueprints/Enum/E_Stat Enum" :default "NewEnumerator0"))
  (returns (Value :type "Float (double-precision)"))
  (return (`BlueprintMapLibrary.Map_Find` (`self.CurrentStats`) Key)))

(fn `GetMaxStatValue`
  (params (Stat :type "/Game/CombatSystem/Blueprints/Enum/E_Stat Enum" :default "NewEnumerator0"))
  (returns (`Max Value` :type "Float (double-precision)"))
  (return (`.MaxValue_4_8B2F8F874DFE4F4D0DC64A8C9E1F42D7` (break `/Game/CombatSystem/Blueprints/Structures/F_BaseStat` (`BlueprintMapLibrary.Map_Find` (`self.BaseStats`) Stat)))))

(fn `GetMinStatValue`
  (params (Stat :type "/Game/CombatSystem/Blueprints/Enum/E_Stat Enum" :default "NewEnumerator0"))
  (returns (`Min Value` :type "Float (double-precision)"))
  (return (`.MinValue_7_805BAC0A40F0651BFA7BC3995B5F630A` (break `/Game/CombatSystem/Blueprints/Structures/F_BaseStat` (`BlueprintMapLibrary.Map_Find` (`self.BaseStats`) Stat)))))

(fn `InitializeStats`
  (bind _keys (`BlueprintMapLibrary.Map_Keys` (`self.BaseStats`)))
  (for _array_element _keys
    (`self.SetCurrentStatValue` _array_element (break `/Game/CombatSystem/Blueprints/Structures/F_BaseStat` (`BlueprintMapLibrary.Map_Find` (`self.BaseStats`) _array_element)))))

(fn `RegenStamina`
  (`self.AddCurrentStatValue` "NewEnumerator2" (`self.StaminaRegenRate`))
  (if (>= (`self.GetCurrentStatValue` "NewEnumerator2") (`self.GetMaxStatValue` "NewEnumerator2"))
    (`KismetSystemLibrary.K2_ClearTimer` null "RegenStamina")))

(fn `SetCurrentStatValue`
  (params (Stat :type "/Game/CombatSystem/Blueprints/Enum/E_Stat Enum" :default "NewEnumerator0") (Value :type "Float (double-precision)"))
  (bind _value (`BlueprintMapLibrary.Map_Find` (`self.BaseStats`) Stat))
  (`BlueprintMapLibrary.Map_Add` (`self.CurrentStats`) Stat (`KismetMathLibrary.FClamp` Value (`.MinValue_7_805BAC0A40F0651BFA7BC3995B5F630A` (break `/Game/CombatSystem/Blueprints/Structures/F_BaseStat` _value)) (`.MaxValue_4_8B2F8F874DFE4F4D0DC64A8C9E1F42D7` (break `/Game/CombatSystem/Blueprints/Structures/F_BaseStat` _value))))
  (`self.OnCurrentStatValueUpdated` (`local.Stat`) (`local.Value`)))

(fn `TakeDamage`
  (params (InDamage :type "Float (double-precision)"))
  (locals (L_DamageFinal :type "Float (double-precision)"))
  (bind _indamage (`local.InDamage`))
  (bind _returnvalue (`Actor.GetComponentByClass` (`self.GetOwner`) "/Game/CombatSystem/Blueprints/Components/AC_StateManagerComponent.AC_StateManagerComponent_C"))
  (bind _output_get (set `local.L_DamageFinal` (* (`local.InDamage`) (/ _indamage (+ _indamage (`self.GetCurrentStatValue` "NewEnumerator3"))))))
  (`self.AddCurrentStatValue` "NewEnumerator1" (* _output_get -1.0))
  (`KismetSystemLibrary.PrintText` (`|FormatText` "in damage : {1}, final damage : {2}" InDamage _output_get))
  (if (<= (`self.GetCurrentStatValue` "NewEnumerator1") 0.0)
    (`/Engine/EditorBlueprintResources/StandardMacros.IsValid` _returnvalue
      (:`Is Valid`
        (`/Game/CombatSystem/Blueprints/Components/AC_StateManagerComponent.SetState` _returnvalue (struct :`TagName` "Character.State.Dead"))))))