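; Actor component that gives its owning character a lock-on targeting toggle for combat.
; Enabling lock-on sphere-traces along the camera's forward vector for an actor that implements BI_Targeting and reports it can be targeted.
; While locked, Tick interpolates the controller's pitch and yaw toward a point below the target's origin, keeping roll, and releases the lock once the target stops being targetable.
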(event `self.ReceiveBeginPlay`
  (bind _ascharacter (cast `Character` (`self.GetOwner`)))
  (set `self.OwnerCharacter` _ascharacter)
  (set `self.OwnerController` (`Pawn.GetController` (`self.OwnerCharacter`)))
  (set `self.OwnerCamera` (`Actor.GetComponentByClass` (`self.OwnerCharacter`) "/Script/Engine.CameraComponent")))

(event `self.ReceiveTick`
  (params (DeltaSeconds :type "Float (single-precision)"))
  (if (`self.bIsTargeting`)
    (`self.UpdateTargetingControlRotation`)))

(event `Enable Lock On`
  (bind (_target _success) (`self.FindTarget`))
  (bind _return_value (message `/Game/CombatSystem/Blueprints/Interfaces/BI_Targeting.CanBeTargeted` _target))
  (if (and _success _return_value)
    (`self.SetTargetActor` _target)
    (`self.SetIsTargeting` true)))

(event `Disable Lock On`
  (`self.SetIsTargeting` false)
  (`self.SetTargetActor` null))

(event `ToggleLockOn`
  (if (`self.bIsTargeting`)
    (`self.Disable Lock On`)
    (else
      (`self.Enable Lock On`))))

(fn `FindTarget`
  (returns (Target :type "Actor Object Reference") (Success :type Boolean))
  (bind (_outhit _returnvalue) (`KismetSystemLibrary.SphereTraceSingleForObjects` (`Actor.K2_GetActorLocation` (`self.GetOwner`)) (+ (`Actor.K2_GetActorLocation` (`self.GetOwner`)) (* (`SceneComponent.GetForwardVector` (`self.OwnerCamera`)) (`self.TargetingDistance`))) (`self.TargetingRadius`) (`self.TargetObjectTypes`) false (`|MakeArray` (`self.GetOwner`)) "ForDuration"))
  (bind (_bblockinghit _binitialoverlap _time _distance _location _impactpoint _normal _impactnormal _physmat _hitactor) (`GameplayStatics.BreakHitResult` _outhit))
  (if (and _returnvalue (`KismetSystemLibrary.IsValid` _hitactor))
    (if (`KismetSystemLibrary.DoesImplementInterface` _hitactor "/Game/CombatSystem/Blueprints/Interfaces/BI_Targeting.BI_Targeting_C")
      (return _hitactor true)
      (else
        _)))
  (return null false))

(fn `GetTargetActor`
  (returns (TargetActor :type "Actor Object Reference"))
  (return (`self.TargetActor`)))

(fn `IsTargeting`
  (returns (bIsTargeting :type Boolean))
  (return (`self.bIsTargeting`)))

(fn `SetIsTargeting`
  (params (bIsTargeting :type Boolean))
  (set `self.bIsTargeting` bIsTargeting))

(fn `SetTargetActor`
  (params (NewTargetActor :type "Actor Object Reference"))
  (set `self.TargetActor` NewTargetActor))

(fn `UpdateTargetingControlRotation`
  (bind (_returnvalue_roll _returnvalue_pitch _returnvalue_yaw) (`KismetMathLibrary.BreakRotator` (`KismetMathLibrary.RInterpTo` (`Actor.K2_GetActorRotation` (`self.OwnerController`)) (`KismetMathLibrary.FindLookAtRotation` (`Actor.K2_GetActorLocation` (`self.GetOwner`)) (- (`Actor.K2_GetActorLocation` (`self.TargetActor`)) (0.0 0.0 100.0))) (`GameplayStatics.GetWorldDeltaSeconds`) (`self.TargetRotationInterpSpeed`))))
  (if (and (`KismetSystemLibrary.IsValid` (`self.OwnerController`)) (`KismetSystemLibrary.IsValid` (`self.TargetActor`)))
    (bind _return_value (message `/Game/CombatSystem/Blueprints/Interfaces/BI_Targeting.CanBeTargeted` (`self.TargetActor`)))
    (if _return_value
      (`Controller.SetControlRotation` (`self.OwnerController`) (`KismetMathLibrary.MakeRotator` (.roll (`Actor.K2_GetActorRotation` (`self.OwnerController`))) _returnvalue_pitch _returnvalue_yaw))
      (else
        (`self.Disable Lock On`)))))