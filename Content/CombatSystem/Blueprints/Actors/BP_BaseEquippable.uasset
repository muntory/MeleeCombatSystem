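; BP_BaseEquippable is a base actor in the combat system for items a Character can equip.
; OnEquipped sets the equipped flag and calls AttachActor, which snaps the item to AttachSocketName on the owning Character's mesh.
; OnUnequipped only clears the flag, without detaching.
; GetItemMesh returns the static mesh component if its mesh is valid, otherwise the skeletal one, as their shared Primitive Component parent type.
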(fn `AttachActor`
  (params (SocketName :type Name))
  (`self.K2_AttachToComponent` (`Character.Mesh` (cast `Character` (`self.GetOwner`) :!pure true)) SocketName "SnapToTarget" "SnapToTarget" "SnapToTarget"))

(fn `GetItemMesh`
  (returns (ReturnValue :type "PrimitiveComponent Object Reference"))
  ;[1 1 1] 스태틱 메쉬와 스켈레탈 메쉬의 부모 클래스인 Primitive Component 로 리턴
  (`/Engine/EditorBlueprintResources/StandardMacros.IsValid` (`StaticMeshComponent.StaticMesh` (`self.ItemStaticMesh`))
    (:`Is Valid`
      (return (`self.ItemStaticMesh`)))
    (:`Is Not Valid`
      (return (`self.ItemSkeletalMesh`)))))

(fn `IsEqupped`
  (returns (ReturnValue :type Boolean))
  (return (`self.bIsEquipped`)))

(fn `OnEquipped`
  (set `self.bIsEquipped` true)
  (`self.AttachActor` (`self.Attach Socket Name`)))

(fn `OnUnequipped`
  (if (`self.bIsEquipped`)
    (set `self.bIsEquipped` false)))

(fn `SetIsEquipped`
  (params (IsEquipped :type Boolean))
  (set `self.bIsEquipped` IsEquipped))

(fn `UserConstructionScript`)