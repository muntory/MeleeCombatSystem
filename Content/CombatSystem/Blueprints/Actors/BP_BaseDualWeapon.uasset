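; Base Blueprint for dual-wielded weapons, extending its parent weapon with a second mesh and its own collision component.
; On equip and combat toggle, the sub weapon snaps to the owning character's hand or stowed socket according to combat state.
; Collision activation and deactivation route to the main or sub weapon component by collision part.
; Sub weapon hits call CanReceiveDamageMessage on the hit actor and apply point damage along the owner's forward vector.
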(event `self.ToggleCombat`
  (params (bIsCombatEnable :type Boolean))
  (`parent.ToggleCombat` bIsCombatEnable)
  (`self.AttachSubWeapon` (select `bool` bIsCombatEnable :`false` (`self.SecondWeaponAttachSocket`) :`true` (`self.SecondWeaponHandSocket`))))

(event `self.SubWeaponColiisionCoponent.OnHit`
  (params (HitResult :type "HitResult Structure"))
  (bind (_bblockinghit _binitialoverlap _time _distance _location _impactpoint _normal _impactnormal _physmat _hitactor) (`GameplayStatics.BreakHitResult` HitResult))
  (message `/Game/CombatSystem/Blueprints/Interfaces/BI_Combat.CanReceiveDamage` _hitactor)
  (`GameplayStatics.ApplyPointDamage` _hitactor (`self.Damage`) (`self.GetActorForwardVector` (`self.GetOwner`)) HitResult (`self.GetInstigatorController`) self))

(fn `ActivateCollision`
  (params (`Collision Part` :type "/Game/CombatSystem/Blueprints/Enum/E_CollisionPart Enum" :default "NewEnumerator0"))
  (switch `/Game/CombatSystem/Blueprints/Enum/E_CollisionPart` `Collision Part`
    (:`NewEnumerator0`
      (`/Game/CombatSystem/Blueprints/Components/AC_CollisionComponent.ActivateCollision` (`self.MainWeaponCollisionComponent`)))
    (:`NewEnumerator1`
      (`/Game/CombatSystem/Blueprints/Components/AC_CollisionComponent.ActivateCollision` (`self.SubWeaponColiisionCoponent`)))))

(fn `AttachSubWeapon`
  (params (SocketName :type Name))
  (`SceneComponent.K2_AttachToComponent` (`self.SubWeaponStaticMesh`) (`Character.Mesh` (cast `Character` (`self.GetOwner`) :!pure true)) SocketName "SnapToTarget" "SnapToTarget" "SnapToTarget" true))

(fn `DeactivateCollision`
  (params (`Collision Part` :type "/Game/CombatSystem/Blueprints/Enum/E_CollisionPart Enum" :default "NewEnumerator0"))
  (switch `/Game/CombatSystem/Blueprints/Enum/E_CollisionPart` `Collision Part`
    (:`NewEnumerator0`
      (`/Game/CombatSystem/Blueprints/Components/AC_CollisionComponent.DeactivateCollision` (`self.MainWeaponCollisionComponent`)))
    (:`NewEnumerator1`
      (`/Game/CombatSystem/Blueprints/Components/AC_CollisionComponent.DeactivateCollision` (`self.SubWeaponColiisionCoponent`)))))

(fn `OnEquipped`
  (`parent.OnEquipped`)
  (`/Game/CombatSystem/Blueprints/Components/AC_CollisionComponent.SetCollisionMesh` (`self.SubWeaponColiisionCoponent`) (`self.SubWeaponStaticMesh`))
  (`self.AttachSubWeapon` (select `bool` (`/Game/CombatSystem/Blueprints/Components/AC_CombatComponent.IsCombatEnable` (`self.CombatComponent`)) :`false` (`self.SecondWeaponAttachSocket`) :`true` (`self.SecondWeaponHandSocket`)))
  (`/Game/CombatSystem/Blueprints/Components/AC_CollisionComponent.AddActorToIgnore` (`self.SubWeaponColiisionCoponent`) (`self.GetOwner`)))

(fn `UserConstructionScript`
  (`parent.UserConstructionScript`))